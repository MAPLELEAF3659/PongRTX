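; Score_player is a goal trigger actor that awards the player a point when a Ball enters its Box.
; On overlap it destroys the ball and increments ScorePlayer on the player pawn, cast to Player.
; When the score reaches the Player's WinScore it shows a "Player Win!" dialog through Player.
; Otherwise it tells the BallSpawner, found by class lookup, to spawn the next ball with a negative argument.
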(event `self.Box.OnComponentBeginOverlap`
  (params (OverlappedComponent :type "PrimitiveComponent Object Reference") (OtherActor :type "Actor Object Reference") (OtherComp :type "PrimitiveComponent Object Reference") (OtherBodyIndex :type Integer) (bFromSweep :type Boolean) (SweepResult :type "HitResult Structure (by ref)"))
  (bind _asball (cast `/Game/Blueprints/Ball` OtherActor))
  (`self.K2_DestroyActor` _asball)
  (bind _asplayer (cast `/Game/Blueprints/Player` (`GameplayStatics.GetPlayerPawn` 0)))
  (bind _returnvalue (`GameplayStatics.GetActorOfClass` "/Game/Blueprints/Player.Player_C"))
  (bind _output_get (set `/Game/Blueprints/Player.Score_player` (+ (`/Game/Blueprints/Player.Score_player` _asplayer) 1) _asplayer))
  (if (>= _output_get (`/Game/Blueprints/Player.WinScore` _returnvalue))
    (bind _returnvalue_2 (`GameplayStatics.GetActorOfClass` "/Game/Blueprints/Player.Player_C"))
    (`/Game/Blueprints/Player.Show Dialog` _returnvalue_2 "Player Win!")
    (else
      (bind _returnvalue_3 (`GameplayStatics.GetActorOfClass` "/Game/Blueprints/BallSpawner.BallSpawner_C"))
      (`/Game/Blueprints/BallSpawner.SpawnNextBall` _returnvalue_3 -1.0))))

(fn `UserConstructionScript`)